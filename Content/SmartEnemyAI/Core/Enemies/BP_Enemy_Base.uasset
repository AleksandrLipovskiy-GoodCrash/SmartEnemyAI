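; BP_Enemy_Base is the base enemy character for the smart enemy AI, providing sword combat actions, a patrol route and movement speed control.
; Attack, wield and sheathe events play montages, then fire end callbacks on completion (attack also on interruption).
; Montage notifies time the weapon spawn onto the hand socket and its destruction when sheathed.
; Getters and setters expose the validated patrol route and map speed states to max walk speed.
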(event Custom|OnAttack
  ;[0.03434 0.03434 0.03434] Attack event
  (Animation|Montage|PlayMontage (Variables|Character|GetMesh) "/Game/SmartEnemyAI/Assets/Enemies/Common/Animations/Combat/Sword/AM_Sword_Normal_Attack.AM_Sword_Normal_Attack"
    (:OnCompleted
      _)
    (:OnInterrupted
      _))
  (Default|CallOnAttackEnd))

(event Custom|OnWieldingWeapon
  ;[0.03434 0.03434 0.03434] Wield Weapon event
  (bind _notifyname (Animation|Montage|PlayMontage (Variables|Character|GetMesh) "/Game/SmartEnemyAI/Assets/Enemies/Common/Animations/Combat/Sword/AM_Sword_Withdrawing_Sword.AM_Sword_Withdrawing_Sword")
    (:OnCompleted
      (Default|CallOnWieldWeapon))
    (:OnNotifyBegin
      (switch name _notifyname
        (:TakeWeapon
          (bind _returnvalue (Game|SpawnActorfromClass "/Game/SmartEnemyAI/Core/Weapons/BP_Weapon_Base.BP_Weapon_Base_C" (Transformation|GetActorTransform) "Undefined" "MultiplyWithRoot" 0 0))
          (bind _output_get (Variables|Weapons|SetWeapon%20In%20Hand _returnvalue))
          (Transformation|AttachComponentToComponent _output_get (Variables|Character|GetMesh) "Weapon_Socket" "SnapToTarget" "SnapToTarget" "SnapToTarget" true)
          (Variables|Weapons|SetbWieldingWeapon true))))))

(event Custom|OnSheathingWeapon
  ;[0.03434 0.03434 0.03434] Reliase Weapon event
  (bind _notifyname (Animation|Montage|PlayMontage (Variables|Character|GetMesh) "/Game/SmartEnemyAI/Assets/Enemies/Common/Animations/Combat/Sword/AM_Sword_Sheathing_Sword.AM_Sword_Sheathing_Sword")
    (:OnCompleted
      (Default|CallOnSheathWeapon))
    (:OnNotifyBegin
      (switch name _notifyname
        (:ReliaseWeapon
          (Actor|DestroyActor (Variables|Weapons|GetWeapon%20In%20Hand))
          (Variables|Weapons|SetbWieldingWeapon false))))))

(fn ConstructionScript)

(fn GetPatrolRoute
  (bind _patrolroute (Variables|AI|GetPatrolRoute)
    (:then
      (return _patrolroute))
    (:else
      (return 0))))

(fn SetMovementSpeed
  (params (Speed :type E_AIMovementSpeed%20Enum :default "NewEnumerator0"))
  (bind _output_get (Variables|/Script/Engine.CharacterMovementComponent|SetMaxWalkSpeed (Variables|Character|GetCharacterMovement) (Utilities|Select :Index Speed :NewEnumerator0 0.0 :NewEnumerator1 (Variables|Movement|GetWalkingSpeed) :NewEnumerator2 (Variables|Movement|GetJoggingSpeed) :NewEnumerator3 (Variables|Movement|GetSprintingSpeed))))
  (return _output_get))