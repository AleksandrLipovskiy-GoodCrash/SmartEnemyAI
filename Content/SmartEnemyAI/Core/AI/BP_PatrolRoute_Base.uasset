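; BP_PatrolRoute_Base is a spline-based patrol route for SmartEnemyAI that tracks the current patrol point.
; OnIncrementPatrolRoute advances PatrolIndex by PatrolDirection and flips the direction at the first and last spline points, producing a ping-pong traversal.
; GetSplinePointAsWorldPosition returns the world location of the PatrolRoute spline point at the current index.
; The index and direction are stored on the route itself.
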(event Custom|OnIncrementPatrolRoute
  (bind _output_get (Variables|PatrolProps|SetPatrolIndex (+ (Variables|PatrolProps|GetPatrolIndex) (Variables|PatrolProps|GetPatrolDirection))))
  (if (== _output_get (- (Spline|GetNumberOfSplinePoints (Variables|Default|GetPatrolRoute)) 1))
    (Variables|PatrolProps|SetPatrolDirection -1)
    (elif (== (Variables|PatrolProps|GetPatrolIndex) 0)
      (Variables|PatrolProps|SetPatrolDirection 1))))

(fn ConstructionScript)

(fn GetSplinePointasWorldPosition
  (return (Spline|GetLocationatSplinePoint (Variables|Default|GetPatrolRoute) (Variables|PatrolProps|GetPatrolIndex) "World")))